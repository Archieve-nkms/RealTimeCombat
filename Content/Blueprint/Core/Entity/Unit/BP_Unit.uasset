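; BP_Unit is a selectable character unit for a game that switches between Tactical and Third Person cameras.
; Selection updates its ground circles, shown only in Tactical mode via a camera-mode event, and writes IsMainUnit to the Blackboard.
; Cursor hover toggles a custom-depth highlight unless the camera is dragging.
; ChangeMesh swaps mesh and AnimClass, then fits capsule and mesh offset by asset name; setters handle walk speed and hold-position state.
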(event `self.ReceiveBeginPlay`
  (`|ExecutionSequence`
    (:`then_0`
      (add `/Game/Blueprint/Core/Player/BP_Player.CamMode switched` (`/Game/Blueprint/Core/Player/BP_PC.Get Player Camera` (`self.Get BP_PC`)) (`|CreateDelegate` :!event `Cam Mode Switch`))
      (set `self.blackBoard` (`AIBlueprintHelperLibrary.GetBlackboard` null))
      (`self.Set Movement Speed` (`self.Walk Speed`)))
    (:`then_1`
      (`self.Update Circles` "NewEnumerator0")
      (`self.Change Mesh` "/Game/Character/Xbot/SM_Xbot.SM_Xbot" "/Game/Character/Animations/ABP_Xbot.ABP_Xbot_C")
      (`self.Set Highlight` false))))

(event `Selected`
  (set `self.IsSelected` true)
  (`self.Update Circles` (`self.Get CamMode`))
  (`BlackboardComponent.SetValueAsBool` (`self.blackBoard`) "IsMainUnit" (`self.Check Unit Is Main Unit`)))

(event `Deselected`
  (set `self.IsSelected` false)
  (`self.Update Circles` (`self.Get CamMode`))
  (`BlackboardComponent.SetValueAsBool` (`self.blackBoard`) "IsMainUnit" false))

(event `self.Mesh.OnBeginCursorOver`
  (params (TouchedComponent :type "PrimitiveComponent Object Reference"))
  (if (not (`/Game/Blueprint/Core/Player/BP_Player.IsDragMode?` (`self.Get Player Camera`)))
    (`self.Set Highlight` true)))

(event `self.Mesh.OnEndCursorOver`
  (params (TouchedComponent :type "PrimitiveComponent Object Reference"))
  (if (not (`/Game/Blueprint/Core/Player/BP_Player.IsDragMode?` (`self.Get Player Camera`)))
    (`self.Set Highlight` false)))

(fn `Cam Mode Switch`
  (params (`new CamMode` :type "/Game/Blueprint/Core/Player/Input/Extra/E_CamMode Enum" :default "NewEnumerator0"))
  (`self.Update Circles` `new CamMode`))

(fn `Change Mesh`
  (params (`new mesh` :type "SkeletalMesh Object Reference") (`new AnimClass` :type "Object Class Reference"))
  (locals (`Capsule Radius` :type "Float (double-precision)" :default 20.0) (`Capsule Half Height` :type "Float (double-precision)" :default 90.0))
  (bind _mesh (`self.Mesh`))
  (bind _capsulecomponent (`self.CapsuleComponent`))
  (bind _capsule_half_height (`local.Capsule Half Height`))
  (`SkeletalMeshComponent.SetAnimInstanceClass` _mesh `new AnimClass`)
  (bind _output_get (set `SkeletalMeshComponent.SkeletalMeshAsset` `new mesh` _mesh))
  (`|ExecutionSequence`
    (:`then_0`
      (switch `string` (`KismetSystemLibrary.GetDisplayName` _output_get)
        (:`Default`
          (set `local.Capsule Radius` 10.0 :!label _label)
          (set `local.Capsule Half Height` 90.0))
        (:`SM_Xbot`
          (goto _label))
        (:`SM_Michelle`
          (set `local.Capsule Radius` 10.0)
          (set `local.Capsule Half Height` 80.0))))
    (:`then_1`
      (`CapsuleComponent.SetCapsuleRadius` _capsulecomponent (`local.Capsule Radius`) true)
      (`CapsuleComponent.SetCapsuleHalfHeight` _capsulecomponent _capsule_half_height true)
      (`SceneComponent.K2_SetRelativeLocation` (`self.Mesh`) (`KismetMathLibrary.MakeVector` 0.0 0.0 (+ (* _capsule_half_height -1.0) -1.65)) false false))))

(fn `Check Unit Is Main Unit`
  (returns (value :type Boolean))
  (return (== self (`/Game/Blueprint/Core/Player/BP_PC.Get Main Unit` (`self.Get BP_PC`)))))

(fn `Get BP_PC`
  (returns (BP_PC :type "/Game/Blueprint/Core/Player/BP_PC Object Reference"))
  (bind _asbp_pc (cast `/Game/Blueprint/Core/Player/BP_PC` (`GameplayStatics.GetPlayerController` 0)))
  (return _asbp_pc))

(fn `Get CamMode`
  (returns (CamMode :type "/Game/Blueprint/Core/Player/Input/Extra/E_CamMode Enum"))
  (return (`/Game/Blueprint/Core/Player/BP_Player.CamMode` (`/Game/Blueprint/Core/Player/BP_PC.Get Player Camera` (`self.Get BP_PC`)))))

(fn `Get Player Camera`
  (returns (`BP Player` :type "/Game/Blueprint/Core/Player/BP_Player Object Reference"))
  (bind _asbp_player (cast `/Game/Blueprint/Core/Player/BP_Player` (`Controller.K2_GetPawn` (`self.Get BP_PC`))))
  (return _asbp_player))

(fn `Set Highlight`
  (params (bValue :type Boolean))
  (`PrimitiveComponent.SetRenderCustomDepth` (`self.Mesh`) bValue))

(fn `Set Hold Position`
  (params (value :type Boolean))
  (set `self.IsHoldingPosition` value))

(fn `Set Movement Speed`
  (params (Speed :type "Float (double-precision)"))
  (set `CharacterMovementComponent.MaxWalkSpeed` Speed (`self.CharacterMovement`)))

(fn `Update Circles`
  (params (`Cam Mode` :type "/Game/Blueprint/Core/Player/Input/Extra/E_CamMode Enum" :default "NewEnumerator0"))
  (bind _select_circle (`self.Select Circle`))
  (bind _display_circle (`self.Display Circle`))
  (switch `/Game/Blueprint/Core/Player/Input/Extra/E_CamMode` `Cam Mode`
    (:`NewEnumerator0`
      (`SceneComponent.SetVisibility` _display_circle true false)
      (`SceneComponent.SetVisibility` _select_circle (`self.IsSelected`) false))
    (:`NewEnumerator1`
      (`SceneComponent.SetVisibility` _display_circle false false)
      (`SceneComponent.SetVisibility` _select_circle false false))))

(fn `UserConstructionScript`)