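; BP_SightBoundary is a helper actor that acts as a detection volume around an owning actor, in the unit entity folder.
; It follows the owner set through SetOwner by copying its location in a self-recalling 0.01-second delay loop instead of attaching or ticking.
; Begin and end overlaps on its SightOverlap component are forwarded to the owner as Found and Lost messages.
; Setters control the visibility and uniform scale of its static mesh.
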(event `self.ReceiveBeginPlay`
  (`self.Follow Owner`))

(event `Follow Owner`
  (bind _owneractor (`self.OwnerActor`))
  (`KismetSystemLibrary.Delay` 0.01)
  (`/Engine/EditorBlueprintResources/StandardMacros.IsValid` _owneractor
    (:`Is Valid`
      (`self.K2_SetActorLocation` (`self.K2_GetActorLocation` _owneractor))
      (`self.Follow Owner`))))

(event `self.SightOverlap.OnComponentBeginOverlap`
  (params (OverlappedComponent :type "PrimitiveComponent Object Reference") (OtherActor :type "Actor Object Reference") (OtherComp :type "PrimitiveComponent Object Reference") (OtherBodyIndex :type Integer) (bFromSweep :type Boolean) (SweepResult :type "HitResult Structure (by ref)"))
  (message `/Game/Blueprint/Interfaces/BPI_Sight.Found` (`self.OwnerActor`) OtherActor))

(event `self.SightOverlap.OnComponentEndOverlap`
  (params (OverlappedComponent :type "PrimitiveComponent Object Reference") (OtherActor :type "Actor Object Reference") (OtherComp :type "PrimitiveComponent Object Reference") (OtherBodyIndex :type Integer))
  (message `/Game/Blueprint/Interfaces/BPI_Sight.Lost` (`self.OwnerActor`) OtherActor))

(fn `Set Boundary Scale`
  (params (Scale :type "Float (double-precision)"))
  (`SceneComponent.SetWorldScale3D` (`self.StaticMesh`) (`KismetMathLibrary.MakeVector` Scale Scale Scale)))

(fn `Set Boundary Visibility`
  (params (value :type Boolean))
  (`SceneComponent.SetVisibility` (`self.StaticMesh`) value false))

(fn `Set Owner`
  (params (Actor :type "Actor Object Reference"))
  (set `self.OwnerActor` Actor))

(fn `UserConstructionScript`)