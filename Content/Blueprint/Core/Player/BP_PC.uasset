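; Player controller for party-based unit control, managing the party roster and unit selection.
; On BeginPlay it limits camera pitch, shows the cursor, adds every BP_Unit to the party and selects the first.
; Selection inserts units by party order, and SwitchUnit deselects all and returns an offset party member with index wrapping.
; It also signals switches between gamepad and keyboard/mouse input, and keys 1 and 2 print debug lists.
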(event `InputAction|KeyDetect` :consume false :paused true
  (params (Key :type "Key Structure"))
  (bind _inputtype (`self.InputType`))
  (:`Pressed`
    (if (`KismetInputLibrary.Key_IsGamepadKey` Key)
      (switch `/Game/Blueprint/Core/Player/Input/Extra/E_InputType` _inputtype
        (:`NewEnumerator0`
          _)
        (:`NewEnumerator1`
          _))
      (set `self.InputType` "NewEnumerator2")
      (else
        (switch `/Game/Blueprint/Core/Player/Input/Extra/E_InputType` _inputtype :!label _label
          (:`NewEnumerator0`
            _)
          (:`NewEnumerator2`
            _))
        (set `self.InputType` "NewEnumerator1")))
    (`self.KeySwitch` (`self.InputType`))))

(event `InputAxis|MouseMove` :consume false :paused true
  (params (AxisValue :type "Float (single-precision)"))
  (if (!= AxisValue 0.0)
    (goto _label)))

(event `self.ReceiveBeginPlay`
  (bind _returnvalue (`GameplayStatics.GetPlayerCameraManager` 0))
  (`|ExecutionSequence`
    (:`then_0`
      (set `PlayerCameraManager.ViewPitchMin` -80.0 _returnvalue)
      (set `PlayerCameraManager.ViewPitchMax` 40.0 _returnvalue)
      (set `self.bShowMouseCursor` true))
    (:`then_1`
      (bind _outactors (`GameplayStatics.GetAllActorsOfClass` "/Game/Blueprint/Core/Entity/Unit/BP_Unit.BP_Unit_C"))
      (for _array_element _outactors
        (bind _asbp_unit (cast `/Game/Blueprint/Core/Entity/Unit/BP_Unit` _array_element))
        (`self.Add unit to party` _asbp_unit))
      ;[1 1 1] Select a first unit in party
      (`self.Select Unit` (`|GetArrayItem` (`self.Units In Party`))))))

(event `Key|One`
  (params (Key :type "Key Structure"))
  (:`Released`
    (for (_array_element _array_index) (`self.Units In Party`)
      (`KismetSystemLibrary.PrintString` (`KismetStringLibrary.Concat_StrStr` (`KismetStringLibrary.Conv_IntToString` _array_index) ": " (`KismetSystemLibrary.GetDisplayName` _array_element))))))

(event `Key|Two`
  (params (Key :type "Key Structure"))
  (:`Released`
    (for (_array_element _array_index) (`self.Selected Units`)
      (`KismetSystemLibrary.PrintString` (`KismetStringLibrary.Concat_StrStr` (`KismetStringLibrary.Conv_IntToString` _array_index) ": " (`KismetSystemLibrary.GetDisplayName` _array_element)) true true (struct :`R` 1.0 :`G` 0.594686 :`B` 0.76969 :`A` 1.0)))))

(fn `Add unit to party`
  (params (`new unit` :type "/Game/Blueprint/Core/Entity/Unit/BP_Unit Object Reference"))
  (`KismetArrayLibrary.Array_AddUnique` (`self.Units In Party`) `new unit`)
  (return))

(fn `Deselect All Units`
  (locals (temp :type "Array of /Game/Blueprint/Core/Entity/Unit/BP_Unit Object Reference"))
  (bind _output_get (set `local.temp` (`self.Selected Units`)))
  (for _array_element _output_get
    (`self.Deselect Unit` _array_element)))

(fn `Deselect Unit`
  (params (`target unit` :type "/Game/Blueprint/Core/Entity/Unit/BP_Unit Object Reference"))
  (bind _returnvalue (`KismetArrayLibrary.Array_RemoveItem` (`self.Selected Units`) `target unit`))
  (`|ExecutionSequence`
    (:`then_0`
      (if _returnvalue
        (`/Game/Blueprint/Core/Entity/Unit/BP_Unit.Deselected` `target unit`)))
    (:`then_1`
      (return))))

(fn `Get Main Unit`
  (returns (`Main Unit` :type "/Game/Blueprint/Core/Entity/Unit/BP_Unit Object Reference"))
  (return (`|GetArrayItem` (`self.Selected Units`))))

(fn `Get Player Camera`
  (returns (`BP Player` :type "/Game/Blueprint/Core/Player/BP_Player Object Reference"))
  (bind _asbp_player (cast `/Game/Blueprint/Core/Player/BP_Player` (`self.K2_GetPawn`)))
  (return _asbp_player))

(fn `Get Unit Index`
  (params (Unit :type "/Game/Blueprint/Core/Entity/Unit/BP_Unit Object Reference"))
  (returns (Index :type Integer))
  (return (`KismetArrayLibrary.Array_Find` (`self.Units In Party`) Unit)))

(fn `Remove unit from party`
  (params (`target unit` :type "/Game/Blueprint/Core/Entity/Unit/BP_Unit Object Reference"))
  (`KismetArrayLibrary.Array_RemoveItem` (`self.Units In Party`) `target unit`)
  (return))

(fn `Select Unit`
  (params (`target unit` :type "/Game/Blueprint/Core/Entity/Unit/BP_Unit Object Reference"))
  (locals (`unit Index In Party` :type Integer) (`target Index` :type Integer :default -1) (targetUnit :type "/Game/Blueprint/Core/Entity/Unit/BP_Unit Object Reference"))
  (bind _targetunit (`local.targetUnit`))
  (bind _selected_units (`self.Selected Units`))
  (set `local.targetUnit` `target unit`)
  (set `local.unit Index In Party` (`KismetArrayLibrary.Array_Find` (`self.Units In Party`) (`local.targetUnit`)))
  (if (`KismetArrayLibrary.Array_Contains` (`self.Selected Units`) (`local.targetUnit`))
    (return)
    (else
      (`|ExecutionSequence`
        (:`then_0`
          (if (== (`local.unit Index In Party`) -1)
            (`KismetArrayLibrary.Array_AddUnique` (`self.Selected Units`) (`local.targetUnit`))
            (else
              (for (_array_element _array_index) (`self.Selected Units`)
                (bind _returnvalue (`KismetArrayLibrary.Array_Find` (`self.Units In Party`) _array_element))
                (if (or (< (`local.unit Index In Party`) _returnvalue) (== _returnvalue -1))
                  (set `local.target Index` _array_index)
                  (break)))
              (if (== (`local.target Index`) -1)
                (`KismetArrayLibrary.Array_AddUnique` _selected_units _targetunit)
                (else
                  (`KismetArrayLibrary.Array_Insert` _selected_units _targetunit (`local.target Index`)))))))
        (:`then_1`
          (`/Game/Blueprint/Core/Entity/Unit/BP_Unit.Selected` (`local.targetUnit`))
          (return))))))

(fn `Switch Unit`
  (params (Amount :type Integer))
  (returns (Success :type Boolean) (Unit :type "/Game/Blueprint/Core/Entity/Unit/BP_Unit Object Reference"))
  (locals (`Start Index` :type Integer))
  (bind _returnvalue (`KismetArrayLibrary.Array_Length` (`self.Units In Party`)))
  (bind _returnvalue_2 (+ Amount (`local.Start Index`)))
  (bind _output_get (set `local.Start Index` (`KismetArrayLibrary.Array_Find` (`self.Units In Party`) (`|GetArrayItem` (`self.Selected Units`)))))
  (if (== _output_get -1)
    (return false (`|GetArrayItem` (`self.Selected Units`)))
    (else
      (`self.Deselect All Units`)
      (return true (`|GetArrayItem` (`self.Units In Party`) (`KismetMathLibrary.SelectInt` (`KismetMathLibrary.SelectInt` _returnvalue_2 (+ _returnvalue_2 _returnvalue) (>= _returnvalue_2 0)) (mod _returnvalue_2 _returnvalue) (== Amount -1)))))))

(fn `Toggle Unit`
  (params (`target unit` :type "/Game/Blueprint/Core/Entity/Unit/BP_Unit Object Reference"))
  (locals (target :type "/Game/Blueprint/Core/Entity/Unit/BP_Unit Object Reference"))
  (bind _target (`local.target`))
  (bind _output_get (set `local.target` `target unit`))
  (if (`/Game/Blueprint/Core/Entity/Unit/BP_Unit.IsSelected` _output_get)
    (`self.Deselect Unit` _target)
    (else
      (`self.Select Unit` _target))))

(fn `UserConstructionScript`)